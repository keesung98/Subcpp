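; TCP client actor that connects to a local server on BeginPlay and receives orientation, speed and depth data.
; Each incoming message is read as a string, printed for debugging, then broken up by chained Split calls into Roll, Pitch, Yaw, Speed and Depth variables.
; The values are only stored here, not applied to anything, and disconnection is not handled.
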(event `self.ReceiveBeginPlay`
  (`self.Connect` "127.0.0.1" 8000 (delegate `Disconnected`) (delegate `Connected`) (delegate `Message_Recv`)))

(event `Disconnected`
  (params (ConnectionId :type Integer)))

(event `Connected`
  (params (ConnectionId :type Integer))
  (if true
    (`KismetSystemLibrary.PrintString` "Connected")))

(event `Message_Recv`
  (params (ConnectionId :type Integer) (Message :type "Array of Byte (by ref)"))
  (`KismetSystemLibrary.PrintString` "Recive Message!")
  (bind _returnvalue (`self.Message_ReadString` Message (`KismetArrayLibrary.Array_Length` Message)))
  (`KismetSystemLibrary.PrintString` _returnvalue true true (struct :`G` 0.66 :`B` 1.0 :`A` 1.0) 100.0)
  (bind _output_get (set `self.SubData` _returnvalue))
  (bind (_lefts _rights) (`KismetStringLibrary.Split` _output_get " "))
  (set `self.Roll` (`KismetStringLibrary.Conv_StringToDouble` _lefts))
  (bind (_lefts_2 _rights_2) (`KismetStringLibrary.Split` _rights " "))
  (set `self.Pitch` (`KismetStringLibrary.Conv_StringToDouble` _lefts_2))
  (bind (_lefts_3 _rights_3) (`KismetStringLibrary.Split` _rights_2 " "))
  (set `self.Yaw` (`KismetStringLibrary.Conv_StringToDouble` _lefts_3))
  (bind (_lefts_4 _rights_4) (`KismetStringLibrary.Split` _rights_3 " "))
  (set `self.Speed` (`KismetStringLibrary.Conv_StringToDouble` _lefts_4))
  (set `self.Depth` (`KismetStringLibrary.Conv_StringToDouble` _rights_4)))

(fn `UserConstructionScript`)