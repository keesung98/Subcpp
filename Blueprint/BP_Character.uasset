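; Character Blueprint whose mesh orientation is driven by roll, pitch and yaw values from a BP_TcpSocket actor.
; BeginPlay casts an Actor variable to BP_TcpSocket and caches the reference.
; Each Tick adds the socket's angles component-wise to the actor's rotation and applies the sum as the mesh's world rotation.
; Debug prints show the current roll, or "none" when the socket reference is invalid.
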(event `self.ReceiveBeginPlay`
  (bind _asbp_tcp_socket (cast `/Game/Blueprint/BP_TcpSocket` (`self.actor`)))
  (set `self.As BP Tcp Socket` _asbp_tcp_socket))

(event `self.ReceiveTick`
  (params (DeltaSeconds :type "Float (single-precision)"))
  (bind (_returnvalue_roll _returnvalue_pitch _returnvalue_yaw) (`KismetMathLibrary.BreakRotator` (`self.K2_GetActorRotation`)))
  (bind _as_bp_tcp_socket (`self.As BP Tcp Socket`))
  (bind _roll (`/Game/Blueprint/BP_TcpSocket.Roll` _as_bp_tcp_socket))
  (`/Engine/EditorBlueprintResources/StandardMacros.IsValid` _as_bp_tcp_socket
    (:`Is Valid`
      (`KismetSystemLibrary.PrintString` (`KismetStringLibrary.Conv_DoubleToString` _roll))
      (`SceneComponent.K2_SetWorldRotation` (`self.Mesh`) (`KismetMathLibrary.MakeRotator` (+ _roll _returnvalue_roll) (+ (`/Game/Blueprint/BP_TcpSocket.Pitch` _as_bp_tcp_socket) _returnvalue_pitch) (+ (`/Game/Blueprint/BP_TcpSocket.Yaw` _as_bp_tcp_socket) _returnvalue_yaw)) false false))
    (:`Is Not Valid`
      (`KismetSystemLibrary.PrintString` "none"))))

(fn `UserConstructionScript`)